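; Player actor that executes move commands from GameManagerActor, stepping forward or back or turning left or right.
; During play, Tick polls the manager and applies each command once as an instant location or rotation change, gated by per-step flags.
; Box overlaps record Ground rotation and detect MoveFloor actors, whose position the player copies while the manager's IsMove is set.
; Outside play, it resets to its BeginPlay location and zero rotation.
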(event `self.ReceiveBeginPlay`
  (set `self.ResetPos` (`self.K2_GetActorLocation`)))

(event `self.ReceiveTick`
  (params (DeltaSeconds :type "Float (single-precision)"))
  (bind _returnvalue (`GameplayStatics.GetActorOfClass` "/Game/BluePrints/Okabe_Blue/GameManagerActor.GameManagerActor_C"))
  (bind _isplay (`/Game/BluePrints/Okabe_Blue/GameManagerActor.GetIsPlayFlag` _returnvalue))
  (if _isplay
    (if (`self.HitMoveFloor`)
      (`self.IsHitMoveFloor` (`self.K2_GetActorLocation` (stale `self.Box.OnComponentBeginOverlap` OtherActor)))
      (else
        (bind _ismove (`/Game/BluePrints/Okabe_Blue/GameManagerActor.GetIsMoveFlag` _returnvalue))
        (if _ismove
          (if (not (`self.MovedFlag`))
            (bind _nowmovedata (`/Game/BluePrints/Okabe_Blue/GameManagerActor.GetNowMoveData` _returnvalue))
            (`self.ChangeMaxMoveTrans` _nowmovedata))
          (elif (`self.ChangedTrans`)
            (set `self.MovedFlag` false)
            (set `self.ChangedTrans` false)))))
    (else
      (`self.InitialzePlayerData`))))

(event `self.Box.OnComponentBeginOverlap`
  (params (OverlappedComponent :type "PrimitiveComponent Object Reference") (OtherActor :type "Actor Object Reference") (OtherComp :type "PrimitiveComponent Object Reference") (OtherBodyIndex :type Integer) (bFromSweep :type Boolean) (SweepResult :type "HitResult Structure (by ref)"))
  (if (`self.ActorHasTag` OtherActor "Ground")
    (set `self.NowRotation` (`self.K2_GetActorRotation` OtherActor))
    (if (`self.InMoveFloor`)
      (set `self.InMoveFloor` false)
      (set `self.HitMoveFloorToCoolTime` false))
    (elif (`self.InMoveFloor`)
      _
      (elif (`self.ActorHasTag` OtherActor "MoveFloor")
        (set `self.HitMoveFloor` true)
        (else
          (set `self.HitMoveFloor` false)
          (`self.K2_SetActorRotation` (`self.NowRotation`)))))))

(fn `ChangeMaxMoveTrans`
  (params (MoveParam :type "/Game/BluePrints/Okabe_Blue/MoveTypeEnum Enum" :default "NewEnumerator1"))
  (bind _returnvalue (`self.K2_GetActorLocation`))
  (bind _returnvalue_2 (`self.K2_GetActorRotation`))
  (bind _addrotat (`self.AddRotat`))
  (bind _roll (.roll _returnvalue_2))
  (bind _pitch (.pitch _returnvalue_2))
  (bind _yaw (.yaw _returnvalue_2))
  (bind _returnvalue_3 (* (`KismetMathLibrary.GetForwardVector` _returnvalue_2) (`self.AddPos`)))
  (if (`self.FrastMove`)
    _
    (elif (not (`self.ChangedTrans`))
      (switch `/Game/BluePrints/Okabe_Blue/MoveTypeEnum` MoveParam
        (:`NewEnumerator1`
          (set `self.MaxMovePos` (+ _returnvalue_3 _returnvalue)))
        (:`NewEnumerator0`
          (set `self.MaxMovePos` (- _returnvalue _returnvalue_3)))
        (:`NewEnumerator2`
          (set `self.MaxMoveRotat` (`KismetMathLibrary.MakeRotator` _roll _pitch (+ _yaw _addrotat))))
        (:`NewEnumerator3`
          (set `self.MaxMoveRotat` (`KismetMathLibrary.MakeRotator` _roll _pitch (- _yaw _addrotat)))))
      (set `self.ChangedTrans` true)
      (`self.MoveState` MoveParam))))

(fn `GetHitMoveFloor`
  (returns (HitMoceFloor :type Boolean))
  (return (`self.HitMoveFloor`)))

(fn `InitialzePlayerData`
  (set `self.MovedFlag` false)
  (`self.K2_SetActorLocation` (`self.ResetPos`))
  (`self.K2_SetActorRotation` (struct))
  (set `self.ChangedTrans` false)
  (set `self.FrastMove` true))

(fn `IsHitMoveFloor`
  (params (MoveActorVec :type "Vector Structure"))
  (bind _returnvalue (`GameplayStatics.GetActorOfClass` "/Game/BluePrints/Okabe_Blue/GameManagerActor.GameManagerActor_C"))
  (if (`/Game/BluePrints/Okabe_Blue/GameManagerActor.IsMove` _returnvalue)
    (`self.K2_SetActorLocation` MoveActorVec)
    (set `self.InMoveFloor` true)
    (elif (`self.HitMoveFloorToCoolTime`)
      (set `self.HitMoveFloor` false)
      (else
        (set `self.HitMoveFloorToCoolTime` true)))))

(fn `MoveState`
  (params (MoveParam :type "/Game/BluePrints/Okabe_Blue/MoveTypeEnum Enum" :default "NewEnumerator1"))
  (switch `/Game/BluePrints/Okabe_Blue/MoveTypeEnum` MoveParam
    (:`NewEnumerator1`
      (`self.前進`))
    (:`NewEnumerator0`
      (`self.後ろ`))
    (:`NewEnumerator2`
      (`self.右`))
    (:`NewEnumerator3`
      (`self.左`))))

(fn `UserConstructionScript`)

(fn `前進`
  (`self.K2_SetActorLocation` (`self.MaxMovePos`) false true))

(fn `右`
  (`self.K2_SetActorRotation` (`self.MaxMoveRotat`)))

(fn `左`
  (`self.K2_SetActorRotation` (`self.MaxMoveRotat`)))

(fn `後ろ`
  (`self.K2_SetActorLocation` (`self.MaxMovePos`)))