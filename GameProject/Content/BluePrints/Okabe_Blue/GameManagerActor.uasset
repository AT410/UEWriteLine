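; GameManagerActor plays back a queued list of move commands for the PlayerActor while IsPlay is set.
; Tick alternates timed move windows, which publish the current MoveData entry, with cooldowns that clear player move flags and advance the index unless HitMoveFloor is set.
; Running past the last entry ends play; while stopped, timers and index are reset, and a sound plays once on the transition from playing to stopped.
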(event `self.ReceiveTick`
  (params (DeltaSeconds :type "Float (single-precision)"))
  (`self.PlayStopSE`)
  (if (`self.IsPlay`)
    (`self.MoveControlle`)
    (`self.CoolTime`)
    (else
      (`self.InitializeManagerData`))))

(fn `CoolTime`
  (if (not (`self.IsMove`))
    (bind _output_get (set `self.NowCoolTime` (+ (`self.NowCoolTime`) (`GameplayStatics.GetWorldDeltaSeconds`))))
    (if (<= _output_get (`self.MaxCoolTime`))
      (set `self.IsMove` false)
      (bind _returnvalue (`GameplayStatics.GetActorOfClass` "/Game/BluePrints/PlayerActor.PlayerActor_C"))
      (set `/Game/BluePrints/PlayerActor.MovedFlag` false _returnvalue)
      (set `/Game/BluePrints/PlayerActor.FrastMove` false _returnvalue)
      (else
        (set `self.NowCoolTime` 0.0)
        (bind _returnvalue_2 (`GameplayStatics.GetActorOfClass` "/Game/BluePrints/PlayerActor.PlayerActor_C"))
        (if (not (`/Game/BluePrints/PlayerActor.HitMoveFloor` _returnvalue_2))
          (set `self.MoveDataItr` (+ (`self.MoveDataItr`) 1)))
        (set `self.IsMove` true)))))

(fn `GetIsMoveFlag`
  (returns (IsMove :type Boolean))
  (return (`self.IsMove`)))

(fn `GetIsPlayFlag`
  (returns (IsPlay :type Boolean))
  (return (`self.IsPlay`)))

(fn `GetNowMoveData`
  (returns (NowMoveData :type "/Game/BluePrints/Okabe_Blue/MoveTypeEnum Enum"))
  (return (`self.NowMoveData`)))

(fn `InitializeManagerData`
  (set `self.IsMove` false)
  (set `self.NowMoveTime` 0.0)
  (set `self.NowCoolTime` 0.0)
  (set `self.MoveDataItr` 0))

(fn `MoveActors`
  (if (not (`self.IsMove`))
    (set `self.IsMove` true)))

(fn `MoveControlle`
  (if (`self.IsMove`)
    (bind _output_get (set `self.NowMoveTime` (+ (`self.NowMoveTime`) (`GameplayStatics.GetWorldDeltaSeconds`))))
    (if (<= _output_get (`self.MaxMoveTime`))
      (if (<= (`self.MoveDataItr`) (`KismetArrayLibrary.Array_LastIndex` (`self.MoveData`)))
        (set `self.NowMoveData` (`|GetArrayItem` (`self.MoveData`) (`self.MoveDataItr`)))
        (bind _returnvalue (`GameplayStatics.GetActorOfClass` "/Game/BluePrints/PlayerActor.PlayerActor_C"))
        (set `/Game/BluePrints/PlayerActor.MovedFlag` false _returnvalue)
        (else
          (set `self.MoveDataItr` 0)
          (set `self.IsMove` false)
          (set `self.IsPlay` false)
          (bind _returnvalue_2 (`GameplayStatics.GetActorOfClass` "/Game/BluePrints/PlayerActor.PlayerActor_C"))
          (set `/Game/BluePrints/PlayerActor.MovedFlag` false _returnvalue_2)))
      (else
        ;[1 1 1] 時間になったら次の行動を取得する
        (set `self.IsMove` false)
        (set `self.NowMoveTime` 0.0)))))

(fn `PlayStopSE`
  (if (`self.IsPlay`)
    (set `self.PlayStopSEFlag` true)
    (elif (`self.PlayStopSEFlag`)
      (`GameplayStatics.PlaySound2D` "/Game/Sound/SE/se_maoudamashii_system20.se_maoudamashii_system20" 1.0 1.0 0.0 null null)
      (set `self.PlayStopSEFlag` false))))

(fn `UserConstructionScript`)