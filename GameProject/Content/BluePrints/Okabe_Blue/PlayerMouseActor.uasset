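; PlayerMouseActor is an actor that runs a debug-drawn line trace on the Visibility channel every tick from its root component.
; The trace end multiplies the root location by the scaled forward vector instead of adding it, so it is not a straight forward ray.
; The hit result drives nothing, the MouseX handlers are empty, and the print and spline-point nodes are disconnected leftovers.
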(event `self.ReceiveTick`
  (params (DeltaSeconds :type "Float (single-precision)"))
  (bind _defaultsceneroot (`self.DefaultSceneRoot`))
  (bind _returnvalue (`SceneComponent.K2_GetComponentLocation` _defaultsceneroot))
  (bind _outhit (`KismetSystemLibrary.LineTraceSingle` :`Start` _returnvalue :`End` (* _returnvalue (* (`KismetMathLibrary.GetForwardVector` (`SceneComponent.K2_GetComponentRotation` _defaultsceneroot)) 1500.0)) :`TraceChannel` "TraceTypeQuery1" :`DrawDebugType` "ForOneFrame" :`bIgnoreSelf` false)))

(event `InputAxisKey|MouseX`
  (params (AxisValue :type "Float (single-precision)")))

(event `InputAxis|MouseX`
  (params (AxisValue :type "Float (single-precision)")))

(fn `UserConstructionScript`)