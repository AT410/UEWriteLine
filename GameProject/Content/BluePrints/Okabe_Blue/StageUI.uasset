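; StageUI is an actor Blueprint that keeps an editable list of move inputs in a MoveData array.
; MoveUp appends the given parameter, BackMoveData removes the last entry and prints the new last index, and ClearMoveData empties the list.
; PlayMove is an empty stub and the event graph has no logic, so nothing here executes the stored moves.
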(fn `BackMoveData`
  (bind _movedata (`self.MoveData`))
  (bind _returnvalue (`KismetArrayLibrary.Array_LastIndex` _movedata))
  (`KismetArrayLibrary.Array_Remove` _movedata _returnvalue)
  (`KismetSystemLibrary.PrintString` (`KismetStringLibrary.Conv_IntToString` _returnvalue)))

(fn `ClearMoveData`
  (`KismetArrayLibrary.Array_Clear` (`self.MoveData`)))

(fn `MoveUp`
  (params (MoveParam :type Integer))
  (`KismetArrayLibrary.Array_Add` (`self.MoveData`) MoveParam))

(fn `PlayMove`)

(fn `UserConstructionScript`)