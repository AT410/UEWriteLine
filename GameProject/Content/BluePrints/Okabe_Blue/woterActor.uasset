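; Water hazard actor that ends play by clearing the GameManagerActor's IsPlay when a Player-tagged actor overlaps its Hit component.
; Each Tick polls the manager's move flag, flipping IsVisible once whenever it drops, using InVisible as a latch, and applying it to the Sphere while it is set.
; When the play flag is off, Tick resets both booleans to false.
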(event `self.ReceiveTick`
  (params (DeltaSeconds :type "Float (single-precision)"))
  (`self.VisibleController`)
  (bind _returnvalue (`GameplayStatics.GetActorOfClass` "/Game/BluePrints/Okabe_Blue/GameManagerActor.GameManagerActor_C"))
  (bind _isplay (`/Game/BluePrints/Okabe_Blue/GameManagerActor.GetIsPlayFlag` _returnvalue))
  (if (not _isplay)
    (set `self.InVisible` false)
    (set `self.IsVisible` false)))

(event `self.Hit.OnComponentBeginOverlap`
  (params (OverlappedComponent :type "PrimitiveComponent Object Reference") (OtherActor :type "Actor Object Reference") (OtherComp :type "PrimitiveComponent Object Reference") (OtherBodyIndex :type Integer) (bFromSweep :type Boolean) (SweepResult :type "HitResult Structure (by ref)"))
  (if (`self.ActorHasTag` OtherActor "Player")
    (bind _returnvalue (`GameplayStatics.GetActorOfClass` "/Game/BluePrints/Okabe_Blue/GameManagerActor.GameManagerActor_C"))
    (set `/Game/BluePrints/Okabe_Blue/GameManagerActor.IsPlay` false _returnvalue)))

(fn `UserConstructionScript`)

(fn `VisibleController`
  (bind _isvisible (`self.IsVisible`))
  (bind _returnvalue (`GameplayStatics.GetActorOfClass` "/Game/BluePrints/Okabe_Blue/GameManagerActor.GameManagerActor_C"))
  (bind _ismove (`/Game/BluePrints/Okabe_Blue/GameManagerActor.GetIsMoveFlag` _returnvalue))
  (if _ismove
    (set `self.InVisible` false)
    (`SceneComponent.SetVisibility` (`self.Sphere`) _isvisible false)
    (elif (not (`self.InVisible`))
      (if _isvisible
        (set `self.IsVisible` false)
        (else
          (set `self.IsVisible` true)))
      (set `self.InVisible` true))))