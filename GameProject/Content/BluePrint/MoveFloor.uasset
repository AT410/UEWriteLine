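; MoveFloor is a moving floor actor that slides along its mesh's forward axis while GameManagerActor's IsMove is set.
; Each Tick during IsPlay it steps a fixed, frame-rate-dependent distance, flips direction once per IsMove activation, and caches its location for GetNowMovePos.
; Outside play it snaps back to its BeginPlay location and clears its flags.
; TargetVector is computed, but only unconnected nodes read it, so nothing limits travel distance.
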(event `self.ReceiveBeginPlay`
  (set `self.moveSpeed` 5)
  (set `self.ResetPosition` (`self.K2_GetActorLocation`)))

(event `self.ReceiveTick`
  (params (DeltaSeconds :type "Float (single-precision)"))
  (bind _returnvalue (`GameplayStatics.GetActorOfClass` "/Game/BluePrints/Okabe_Blue/GameManagerActor.GameManagerActor_C"))
  (if (`/Game/BluePrints/Okabe_Blue/GameManagerActor.IsPlay` _returnvalue)
    (`self.MoveActor`)
    (`self.ChengeTargetVector`)
    (set `self.NowMoveFloor` (`self.K2_GetActorLocation`))
    (else
      (`self.K2_SetActorLocation` (`self.ResetPosition`))
      (set `self.beforeMoveFlg` false)
      (set `self.MoveFlg` false)
      (set `self.IsChengeTargetVector` false))))

(fn `ChengeTargetVector`
  (bind _staticmeshcomponent (`self.StaticMeshComponent`))
  (bind _returnvalue (`SceneComponent.K2_GetComponentLocation` _staticmeshcomponent))
  (bind _returnvalue_2 (`SceneComponent.GetForwardVector` _staticmeshcomponent))
  (bind _returnvalue_3 (`GameplayStatics.GetActorOfClass` "/Game/BluePrints/Okabe_Blue/GameManagerActor.GameManagerActor_C"))
  (if (`/Game/BluePrints/Okabe_Blue/GameManagerActor.IsMove` _returnvalue_3)
    (if (not (`self.IsChengeTargetVector`))
      (if (`self.beforeMoveFlg`)
        (set `self.targetVector` (+ (* (`KismetMathLibrary.Normal` _returnvalue_2) 200) _returnvalue))
        (else
          (set `self.targetVector` (+ (* (`KismetMathLibrary.Normal` _returnvalue_2) -200) _returnvalue))))
      (if (`self.beforeMoveFlg`)
        (set `self.beforeMoveFlg` false)
        (set `self.MoveFlg` true)
        (else
          (set `self.beforeMoveFlg` true)
          (set `self.MoveFlg` false)))
      (set `self.IsChengeTargetVector` true))
    (else
      (set `self.IsChengeTargetVector` false))))

(fn `GetNowMovePos`
  (returns (MoveFloorPos :type "Vector Structure"))
  (return (`self.NowMoveFloor`)))

(fn `MoveActor`
  (bind _staticmeshcomponent (`self.StaticMeshComponent`))
  (bind _returnvalue (`SceneComponent.GetForwardVector` _staticmeshcomponent))
  (bind _returnvalue_2 (`SceneComponent.K2_GetComponentLocation` _staticmeshcomponent))
  (bind _returnvalue_3 (`GameplayStatics.GetActorOfClass` "/Game/BluePrints/Okabe_Blue/GameManagerActor.GameManagerActor_C"))
  (if (`/Game/BluePrints/Okabe_Blue/GameManagerActor.IsMove` _returnvalue_3)
    (if (`self.MoveFlg`)
      (`self.K2_SetActorLocation` (+ (* _returnvalue (`self.moveSpeed`)) _returnvalue_2))
      (else
        (`self.K2_SetActorLocation` (+ _returnvalue_2 (* _returnvalue (* (`self.moveSpeed`) -1.0))))))))

(fn `UserConstructionScript`)